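; Destructible 1M cube actor that shatters after something overlaps it long enough.
; Overlap events toggle a flag that lets Tick count Timer down by Remover each frame, independent of delta time, without resetting it.
; Once Timer runs out, the destructible mesh enables physics and applies huge radius damage to itself at its own location.
; A Remove event also decrements the timer directly.
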(event Custom|Remove
  (Variables|Default|SetTimer (- (Variables|Default|GetTimer) (Variables|Default|Getremover))))

(event Collision|EventActorBeginOverlap
  (params (OtherActor :type Actor%20Object%20Reference))
  (bind _1m_cube_dm (Variables|Default|Get1M_Cube_DM))
  (Variables|Default|SetIsde true)
  (if (<= (Variables|Default|GetTimer) 0.0)
    (Physics|SetSimulatePhysics _1m_cube_dm true)
    (Class|DestructibleComponent|ApplyRadiusDamage _1m_cube_dm 3e+07 (Transformation|GetWorldLocation _1m_cube_dm) 0.0 3e+03 true)
    (else
      (Variables|Default|SetTimer (- (Variables|Default|GetTimer) (Variables|Default|Getremover))))))

(event Collision|EventActorEndOverlap
  (params (OtherActor :type Actor%20Object%20Reference))
  (Variables|Default|SetIsde false))

(event EventTick
  (params (DeltaSeconds :type Float%20%28single-precision%29))
  (bind _1m_cube_dm (Variables|Default|Get1M_Cube_DM))
  (if (Variables|Default|GetIsde)
    (if (<= (Variables|Default|GetTimer) 0.0)
      (Physics|SetSimulatePhysics _1m_cube_dm true)
      (Class|DestructibleComponent|ApplyRadiusDamage _1m_cube_dm 3e+07 (Transformation|GetWorldLocation _1m_cube_dm) 0.0 3e+03 true)
      (else
        (Variables|Default|SetTimer (- (Variables|Default|GetTimer) (Variables|Default|Getremover)))))))

(fn ConstructionScript)